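; Footstep anim notify that plays a surface-specific sound and Niagara effect at a configurable mesh socket.
; On notify, it traces downward from the socket on the Visibility channel, ignoring the owner, and reads the hit physical material's surface type.
; CheckSurfaceType maps that surface to run SFX and VFX assets, using tile audio and its effect as the default.
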(fn ReceivedNotify
  (params (MeshComp :type Skeletal%20Mesh%20Component%20Object%20Reference) (Animation :type Anim%20Sequence%20Base%20Object%20Reference) (EventReference :type Anim%20Notify%20Event%20Reference%20Structure%20%28by%20ref%29))
  (bind _socketname (Variables|Default|GetSocketName))
  (bind _returnvalue (Transformation|GetSocketLocation MeshComp _socketname))
  (bind _outhit (Collision|LineTraceByChannel _returnvalue (+ _returnvalue "0.000000,0.000000,-400.000000") "TraceTypeQuery1" false (Utilities|Array|MakeArray (Components|GetOwner MeshComp)) "None"))
  (|CheckSurfaceType (Variables|/Script/PhysicsCore.PhysicalMaterial|GetSurfaceType (.physmat _outhit))
    (:then
      _)
    (:then2
      _)
    (:then3
      _)
    (:then4
      _)
    (:then5
      _)
    (:then6
      _)
    (:then7
      _))
  (Audio|PlaySoundatLocation (LocalVariables|GetSFX) _returnvalue "0, 0, 0" 1.0 1.0 0.0 0 0 0 0)
  (Niagara|SpawnSystematLocation (LocalVariables|GetVFX) _returnvalue)
  (return false))