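; BP_BossZone is a trigger actor that engages a referenced boss when the player enters its area.
; On overlap by the player character, it sets that player as the Boss's target and shows the Boss's overlay widget on screen.
; When the player leaves, it clears the target and removes the overlay, doing nothing if the Boss reference is invalid.
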(event Collision|EventActorBeginOverlap
  (params (OtherActor :type Actor%20Object%20Reference))
  (bind _boss (Variables|Default|GetBoss))
  (bind _asbp_player_character (Utilities|Casting|CastToBP_PlayerCharacter (Game|GetPlayerCharacter 0)))
  (if (== _asbp_player_character OtherActor)
    (Utilities|IsValid _boss
      (:Is%20Valid
        (Class|CBEnemyCharacter|SetTargetActor _boss _asbp_player_character)
        (UserInterface|Viewport|AddtoViewport (Variables|/Script/Combat.CB_EnemyCharacter|GetBossOverlay _boss) 0)))))

(event Collision|EventActorEndOverlap
  (params (OtherActor :type Actor%20Object%20Reference))
  (bind _boss (Variables|Default|GetBoss))
  (bind _asbp_player_character (Utilities|Casting|CastToBP_PlayerCharacter (Game|GetPlayerCharacter 0)))
  (if (== _asbp_player_character OtherActor)
    (Utilities|IsValid _boss
      (:Is%20Valid
        (Class|CBEnemyCharacter|SetTargetActor _boss)
        (Widget|RemovefromParent (Variables|/Script/Combat.CB_EnemyCharacter|GetBossOverlay _boss))))))

(fn ConstructionScript)