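; BP_SwordEnemy is a sword enemy Blueprint whose Dead event is empty.
; An unconnected chain holds boss-defeat logic that never runs: it marks the level cleared in CB_GameInstance, stops the AI, removes the boss overlay and increments the win count.
; The same dormant chain then waits briefly and spawns a BP_Teleport below the actor's location.
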(event EventDead)

(fn ConstructionScript)